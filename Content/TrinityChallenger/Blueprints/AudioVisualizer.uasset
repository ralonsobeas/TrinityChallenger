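; AudioVisualizer is a component for a Post Process Volume that turns an Intensity value into a screen-wide visual pulse.
; On BeginPlay it caches the owning volume's settings.
; Each Tick it linearly maps Intensity to a subtle film Slope offset and a stronger DetailStrength scale, then writes the settings back to the volume.
; Intensity is only read here, with no audio analysis in this graph.
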(event `self.ReceiveBeginPlay`
  (bind _asvolumen_de_post_procesamiento (cast `PostProcessVolume` (`self.GetOwner`)))
  (set `self.PostProcessSetting` (`PostProcessVolume.Settings` _asvolumen_de_post_procesamiento)))

(event `self.ReceiveTick`
  (params (DeltaSeconds :type "Float (single-precision)"))
  (bind _intensity (`self.Intensity`))
  (bind _asvolumen_de_post_procesamiento (cast `PostProcessVolume` (`self.GetOwner`)))
  (bind _structout (setmembers `PostProcessSettings` :`StructRef` (`self.PostProcessSetting`) :`FilmSlope` (+ (/ (- _intensity 0.5) 20.0) 0.65) :`LocalExposureDetailStrength` (* _intensity 4.0)))
  (set `PostProcessVolume.Settings` _structout _asvolumen_de_post_procesamiento))
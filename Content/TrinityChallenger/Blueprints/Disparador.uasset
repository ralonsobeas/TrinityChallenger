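; Disparador is a weapon firing component that resolves hitscan shots and triggers the end menu when the player is hit.
; Tick consumes the Shoot flag when ready, line-tracing from externally set origin and direction while held, ignoring the weapon's owner.
; Hits flag targets' Morir component; non-player shots briefly show a bullet at impact.
; A second trace after the sound detects player hits or re-arms firing; Revive clears shot state.
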(event `self.ReceiveBeginPlay`
  (bind _returnvalue (`self.GetOwner`))
  (bind _returnvalue_2 (`Actor.GetParentActor` _returnvalue))
  ;[1 1 1] Ajustar para actores a ignorar en el disparo (no autodisparo)
  (`/Engine/EditorBlueprintResources/StandardMacros.IsValid` _returnvalue_2
    (:`Is Valid`
      (set `self.WeaponOwner` _returnvalue_2))
    (:`Is Not Valid`
      (set `self.WeaponOwner` _returnvalue))))

(event `self.ReceiveTick`
  (params (DeltaSeconds :type "Float (single-precision)"))
  (bind _shootorigin (`self.ShootOrigin`))
  ;[1 1 1] Check Input para Disparar
  (if (`self.waitForShotToEnd`)
    (if (`self.Shoot`)
      (set `self.waitForShotToEnd` false)
      (set `self.Shoot` false)
      ;[1 1 1] Crear Raycast
      (if (`self.IsWeaponBeingHeld`)
        (bind _outhit (`self.CrearRaycast`))
        (bind (_bblockinghit _binitialoverlap _time _distance _location _impactpoint _normal _impactnormal _physmat _hitactor) (`GameplayStatics.BreakHitResult` _outhit))
        (bind _returnvalue (`Actor.GetComponentByClass` _hitactor "/Game/TrinityChallenger/Blueprints/Morir.Morir_C"))
        ;[1 1 1] Matar lo que toque (En caso de IA)
        (`/Engine/EditorBlueprintResources/StandardMacros.IsValid` _returnvalue
          (:`Is Valid`
            (set `/Game/TrinityChallenger/Blueprints/Morir.Hit` true _returnvalue))
          (:`Is Not Valid`
            _))
        ;[1 1 1] En caso de que el disparo no sea de jugador ignoramos bala
        (if (not (== (`self.WeaponOwner`) (`GameplayStatics.GetPlayerPawn` 0)))
          ;[1 1 1] Crear bala, reproducir sonido y eliminar bala
          (bind _returnvalue_2 (`|SpawnActorFromClass` "/Game/TrinityChallenger/Blueprints/Bullet.Bullet_C" (`KismetMathLibrary.MakeTransform` (- _impactpoint (* (`KismetMathLibrary.Normal` (- _impactpoint _shootorigin)) 10.0)) (`KismetMathLibrary.FindLookAtRotation` _shootorigin (`self.ShootDirection`))) "Undefined" "OverrideRootScale" null null))
          (`KismetSystemLibrary.Delay` 0.5)
          (`Actor.K2_DestroyActor` _returnvalue_2))
        (`GameplayStatics.PlaySoundAtLocation` "/Game/StarterContent/Audio/Explosion02.Explosion02" (`self.ShootOrigin`) (struct) 1.0 1.0 0.0 null null null null)
        ;[1 1 1] Segundo raycast
        (bind _outhit_2 (`self.CrearRaycast`))
        ;[1 1 1] Check objetivo es player
        (if (== (`GameplayStatics.GetPlayerPawn` 0) (`.HitActor` (`GameplayStatics.BreakHitResult` _outhit_2)))
          (bind _returnvalue_3 (`GameplayStatics.GetActorOfClass` "/Game/ThirdPerson/Blueprints/BP_ThirdPersonCharacter.BP_ThirdPersonCharacter_C"))
          (`self.ShowFinalMenu` _returnvalue_3)
          (else
            ;[1 1 1] No acierta -> Siguiente disparo
            (set `self.waitForShotToEnd` true)))))
    (else
      (set `self.Shoot` false))))

(fn `CrearRaycast`
  (returns (OutHit :type "HitResult Structure"))
  (bind _shootorigin (`self.ShootOrigin`))
  (bind _outhit (`KismetSystemLibrary.LineTraceSingle` _shootorigin (+ _shootorigin (`self.ShootDirection`)) "TraceTypeQuery1" false (`|MakeArray` (`self.WeaponOwner`)) "ForDuration" true (struct :`R` 1.0 :`A` 1.0) (struct :`G` 1.0 :`A` 1.0) 0.5))
  (return _outhit))

(fn `Revive`
  (set `self.Shoot` false)
  (set `self.waitForShotToEnd` false)
  (set `self.ShootDirection` (0.0 0.0 0.0))
  (set `self.ShootOrigin` (0.0 0.0 0.0)))

(fn `ShowFinalMenu`
  (params (self2 :type "/Game/ThirdPerson/Blueprints/BP_ThirdPersonCharacter Object Reference"))
  (bind _returnvalue (`GameplayStatics.GetPlayerController` 0))
  (bind _interfazjuego (`/Game/ThirdPerson/Blueprints/BP_ThirdPersonCharacter.InterfazJuego` self2))
  ;[1 1 1] Si dispara a jugador abre menú "THE END" donde se sale del juego
  (`Widget.SetVisibility` (`/Game/TrinityChallenger/Interface/InterfazJuego.EndText` _interfazjuego) "Visible")
  (`Widget.SetVisibility` (`/Game/TrinityChallenger/Interface/InterfazJuego.ExitButton` _interfazjuego) "Visible")
  (`Widget.SetVisibility` (`/Game/TrinityChallenger/Interface/InterfazJuego.CheckpointButton` _interfazjuego) "Visible")
  (`Widget.SetVisibility` (`/Game/TrinityChallenger/Interface/InterfazJuego.RestartButton` _interfazjuego) "Visible")
  (set `/Game/TrinityChallenger/Interface/InterfazJuego.TextBlockUpdate` false _interfazjuego)
  (set `PlayerController.bShowMouseCursor` true _returnvalue)
  (`WidgetBlueprintLibrary.SetInputMode_UIOnlyEx` _returnvalue _interfazjuego))
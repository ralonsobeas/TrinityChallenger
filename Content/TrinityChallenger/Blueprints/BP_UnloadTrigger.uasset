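; BP_UnloadTrigger is a box trigger that shows or hides lights and static mesh actors as the player enters or leaves its area.
; On BeginPlay it briefly shrinks and restores the box to force overlaps, and caches all triggers of its class.
; Overlapping static meshes and "Light"-tagged actors register for visibility toggling.
; On exit it hides them, then re-shows those of any trigger still flagged as occupied, so overlapping areas stay visible.
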(event `self.ReceiveBeginPlay`
  (bind _box (`self.Box`))
  ;[1 1 1] Asegurar que haya colision al inicio del juego
  (bind _output_get (set `self.auxVector` (`SceneComponent.K2_GetComponentToWorld` (`self.Box`))))
  (`SceneComponent.K2_SetWorldTransform` _box (`KismetMathLibrary.MakeTransform` (.location _output_get) (.rotation _output_get) (0.1 0.1 0.1)) false false)
  (`KismetSystemLibrary.Delay` 0.1)
  (`SceneComponent.K2_SetWorldTransform` _box _output_get false false)
  (bind _outactors (`GameplayStatics.GetAllActorsOfClass` "BP_UnloadTrigger_C"))
  (set `self.OtherUnloaders` _outactors))

(event `self.ReceiveActorBeginOverlap`
  (params (OtherActor :type "Actor Object Reference"))
  ;[1 1 1] Añadir luces que choquen al array
  (cast `StaticMeshActor` OtherActor
    (:`then`
      (`KismetArrayLibrary.Array_AddUnique` (`self.LightsToLoad`) OtherActor :!label _label))
    (:`CastFailed`
      (if (`self.ActorHasTag` OtherActor "Light")
        (goto _label)
        (else
          ;[1 1 1] Si el jugador entra en la zona cargamos las luces
          (`self.Execute If Object Is Player` OtherActor)
          (bind _output_get (set `self.isPlayerinArea` true))
          (`self.Ajustar Visibilidad Luces` _output_get))))))

(event `self.ReceiveActorEndOverlap`
  (params (OtherActor :type "Actor Object Reference"))
  ;[1 1 1] Si el jugador sale de la zona desactivamos las luces
  (`self.Execute If Object Is Player` OtherActor)
  (bind _output_get (set `self.isPlayerinArea` false))
  (`self.Ajustar Visibilidad Luces` _output_get)
  ;[1 1 1] Activamos las luces que estuvieran en otro area del que el jugador no haya salido
  (for _array_element (`self.OtherUnloaders`)
    (if (`/Game/TrinityChallenger/Blueprints/BP_UnloadTrigger.isPlayerinArea` _array_element)
      (`self.Ajustar Visibilidad Luces` _array_element true))))

(fn `Ajustar Visibilidad Luces`
  (params (`Valor Luz` :type Boolean))
  (for _array_element (`self.LightsToLoad`)
    (`/Engine/EditorBlueprintResources/StandardMacros.IsValid` _array_element
      (:`Is Valid`
        (`SceneComponent.SetVisibility` (`Actor.RootComponent` _array_element) `Valor Luz` true)))))

(fn `Execute If Object Is Player`
  (params (Object :type "Actor Object Reference"))
  (if (== Object (`GameplayStatics.GetPlayerPawn` 0))
    (return)))

(fn `UserConstructionScript`)
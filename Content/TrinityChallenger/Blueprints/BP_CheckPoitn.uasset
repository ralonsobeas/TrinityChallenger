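; BP_CheckPoitn is a one-shot checkpoint trigger that fires the first time the player pawn overlaps it.
; It gathers every AI_Character whose Morir component is not dead into a list of living enemies and saves each one's location as that component's starting position.
; It then registers itself as the third-person character's current checkpoint and stores its own location as the player position.
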(event `self.ReceiveActorBeginOverlap`
  (params (OtherActor :type "Actor Object Reference"))
  (if (not (`self.oneTimeExecute`))
    (bind _exec (`self.Execute if object is player` OtherActor))
    (if _exec
      (set `self.oneTimeExecute` true)
      (bind _outactors (`GameplayStatics.GetAllActorsOfClass` "/Game/TrinityChallenger/AI/AI_Character.AI_Character_C"))
      (for _array_element _outactors
        (bind _returnvalue (`self.GetComponentByClass` _array_element "/Game/TrinityChallenger/Blueprints/Morir.Morir_C"))
        (if (not (`/Game/TrinityChallenger/Blueprints/Morir.isDead` _returnvalue))
          (`KismetArrayLibrary.Array_AddUnique` (`self.CurrentAliveEnemies`) _array_element)
          (set `/Game/TrinityChallenger/Blueprints/Morir.startingPosition` (`self.K2_GetActorLocation` _array_element) _returnvalue)))
      (bind _asbp_third_person_character (cast `/Game/ThirdPerson/Blueprints/BP_ThirdPersonCharacter` (`GameplayStatics.GetPlayerPawn` 0)))
      (bind _output_get (set `/Game/ThirdPerson/Blueprints/BP_ThirdPersonCharacter.currentCheckpoint` self _asbp_third_person_character))
      (set `self.PlayerPos` (`self.K2_GetActorLocation` _output_get)))))

(fn `Execute if object is player`
  (params (Object :type "Actor Object Reference"))
  (returns (exec :type Boolean))
  (bind _returnvalue (== Object (`GameplayStatics.GetPlayerPawn` 0)))
  (if _returnvalue
    (return _returnvalue)))

(fn `UserConstructionScript`)
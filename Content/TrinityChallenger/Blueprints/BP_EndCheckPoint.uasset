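; End checkpoint trigger that ends the run with a victory screen when the player reaches it.
; On the first overlap by the local player pawn, it reveals the end text, exit and restart buttons on the player's game HUD widget.
; It shows a final score adding the displayed score text to ten points per enemy killed, stops the text updates and switches to UI-only input with the cursor shown.
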(event `self.ReceiveActorBeginOverlap`
  (params (OtherActor :type "Actor Object Reference"))
  (if (not (`self.One Time Execute`))
    (bind _exec (`self.Execute if object is player` OtherActor))
    (if _exec
      (set `self.One Time Execute` true)
      (bind _asbp_third_person_character (cast `/Game/ThirdPerson/Blueprints/BP_ThirdPersonCharacter` OtherActor))
      (`self.Show Final Menu` _asbp_third_person_character))))

(fn `Execute if Object is Player`
  (params (Object :type "Actor Object Reference"))
  (returns (exec :type Boolean))
  (bind _returnvalue (== Object (`GameplayStatics.GetPlayerPawn` 0)))
  (if _returnvalue
    (return _returnvalue)))

(fn `Show Final Menu`
  (params (player :type "/Game/ThirdPerson/Blueprints/BP_ThirdPersonCharacter Object Reference"))
  (bind _returnvalue (`GameplayStatics.GetPlayerController` 0))
  (bind _interfazjuego (`/Game/ThirdPerson/Blueprints/BP_ThirdPersonCharacter.InterfazJuego` player))
  (bind _points (`/Game/TrinityChallenger/Interface/InterfazJuego.Points` _interfazjuego))
  (bind _endtext (`/Game/TrinityChallenger/Interface/InterfazJuego.EndText` _interfazjuego))
  (bind _returnvalue_2 (`KismetTextLibrary.Conv_TextToString` (`TextBlock.GetText` (`/Game/TrinityChallenger/Interface/InterfazJuego.TextBlock_0` _interfazjuego))))
  ;[1 1 1] Si dispara a jugador abre menú "THE END" donde se sale del juego
  (`TextBlock.SetText` _endtext "VICTORY")
  (`Widget.SetVisibility` _endtext "Visible")
  (`Widget.SetVisibility` (`/Game/TrinityChallenger/Interface/InterfazJuego.ExitButton` _interfazjuego) "Visible")
  (bind _returnvalue_3 (`GameplayStatics.GetActorOfClass` "/Game/ThirdPerson/Blueprints/BP_ThirdPersonCharacter.BP_ThirdPersonCharacter_C"))
  (bind _enemieskilled (`/Game/ThirdPerson/Blueprints/BP_ThirdPersonCharacter.enemiesKilled` _returnvalue_3))
  (`TextBlock.SetText` _points (`KismetTextLibrary.Conv_StringToText` (`KismetStringLibrary.Concat_StrStr` "SCORE: " _returnvalue_2 " + " (`KismetStringLibrary.Conv_IntToString` _enemieskilled) " x " "10 = " (`KismetStringLibrary.Conv_DoubleToString` (+ (`KismetStringLibrary.Conv_StringToDouble` _returnvalue_2) (* _enemieskilled 10))))))
  (`Widget.SetVisibility` _points "Visible")
  (`Widget.SetVisibility` (`/Game/TrinityChallenger/Interface/InterfazJuego.RestartButton` _interfazjuego) "Visible")
  (set `/Game/TrinityChallenger/Interface/InterfazJuego.TextBlockUpdate` false _interfazjuego)
  (set `PlayerController.bShowMouseCursor` true _returnvalue)
  (`WidgetBlueprintLibrary.SetInputMode_UIOnlyEx` _returnvalue _interfazjuego))

(fn `UserConstructionScript`)
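; AIShoot is a component that makes an AI enemy shoot at the player.
; On BeginPlay it caches the player, the owner's Disparador shooter component and the attached weapon.
; Each tick, while alive and after the player grabs a first weapon, a debug-drawn line trace checks visibility.
; Sight switches the mesh to idle and fires Disparador along the weapon arrow's forward vector; losing sight switches to a walk loop.
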(event `self.ReceiveBeginPlay`
  (bind _returnvalue (`self.GetOwner`))
  ;[1 1 1] Guardamos Jugador
  (bind _returnvalue_2 (`GameplayStatics.GetActorOfClass` "/Game/ThirdPerson/Blueprints/BP_ThirdPersonCharacter.BP_ThirdPersonCharacter_C"))
  (set `self.Player` _returnvalue_2)
  ;[1 1 1] Guardamos componente disparador
  (set `self.Disparador` (`Actor.GetComponentByClass` _returnvalue "/Game/TrinityChallenger/Blueprints/Disparador.Disparador_C"))
  ;[1 1 1] Guardamos el arma de la IA
  (for _array_element (`Actor.GetAttachedActors` _returnvalue true false)
    (bind _asbp_weapon (cast `/Game/TrinityChallenger/Blueprints/BP_Weapon` _array_element))
    (set `self.Weapon` _asbp_weapon)))

(event `self.ReceiveTick`
  (params (DeltaSeconds :type "Float (single-precision)"))
  (bind _returnvalue (`self.GetOwner`))
  (bind _returnvalue_2 (`self.GetOwner`))
  (bind _disparador (`self.Disparador`))
  (bind _animationhelper (`self.animationHelper`))
  (bind _returnvalue_3 (`Actor.GetComponentByClass` (`self.Weapon`) "/Script/Engine.ArrowComponent"))
  ;[1 1 1] Condiciones de disparo
  (if (`/Game/ThirdPerson/Blueprints/BP_ThirdPersonCharacter.grabbedFirstWeapon` (`self.Player`))
    (if (not (`self.isDead`))
      ;[1 1 1] Comprobamos que la IA tenga visión con el jugador
      (bind _outhit (`KismetSystemLibrary.LineTraceSingle` (`SceneComponent.K2_GetComponentLocation` (`Actor.GetComponentByClass` _returnvalue_2 "/Script/Engine.ArrowComponent")) (`Actor.K2_GetActorLocation` (`self.Player`)) "TraceTypeQuery1" false (`|MakeArray` _returnvalue_2) "ForOneFrame" true (struct :`R` 1.0 :`B` 0.846352 :`A` 1.0) (struct :`R` 1.0 :`G` 0.871338 :`A` 1.0)))
      (cast `/Game/ThirdPerson/Blueprints/BP_ThirdPersonCharacter` (`.HitActor` (`GameplayStatics.BreakHitResult` _outhit))
        (:`then`
          ;[1 1 1] Ajustamos animacion dependiendo de si vemos o no al jugador (FALTA ANIMACION APUNTAR)
          (if _animationhelper
            (set `self.animationHelper` false)
            (bind _asactor_de_malla_del_esqueleto (cast `SkeletalMeshActor` _returnvalue))
            (`SkeletalMeshComponent.PlayAnimation` (`SkeletalMeshActor.SkeletalMeshComponent` _asactor_de_malla_del_esqueleto) "/Game/MCO_Mocap_Basics/Animation/Mobility_Pro/Root_Motion/MOB1_Stand_Relaxed_Idle_v2.MOB1_Stand_Relaxed_Idle_v2" true))
          ;[1 1 1] Ajustamos variables y disparamos
          (set `/Game/TrinityChallenger/Blueprints/Disparador.ShootOrigin` (`SceneComponent.K2_GetComponentLocation` _returnvalue_3) _disparador)
          (set `/Game/TrinityChallenger/Blueprints/Disparador.ShootDirection` (* (`KismetMathLibrary.GetForwardVector` (`SceneComponent.K2_GetComponentRotation` _returnvalue_3)) 3000) _disparador)
          (set `/Game/TrinityChallenger/Blueprints/Disparador.IsWeaponBeingHeld` true _disparador)
          (set `/Game/TrinityChallenger/Blueprints/Disparador.Shoot` true _disparador))
        (:`CastFailed`
          (if (not _animationhelper)
            (set `self.animationHelper` true)
            (bind _asactor_de_malla_del_esqueleto_2 (cast `SkeletalMeshActor` _returnvalue))
            (`SkeletalMeshComponent.PlayAnimation` (`SkeletalMeshActor.SkeletalMeshComponent` _asactor_de_malla_del_esqueleto_2) "/Game/MCO_Mocap_Basics/Animation/Walks/Root_Motion/Walk_13_Power_Walk_Loop.Walk_13_Power_Walk_Loop" true)))))))

(fn `GetRandomVector`
  (params (Range :type "Float (double-precision)"))
  (returns (Vector :type "Vector Structure"))
  (bind _returnvalue (* Range 2.0))
  (return (`KismetMathLibrary.MakeVector` (* (- (`KismetMathLibrary.RandomFloat`) 0.5) _returnvalue) (* (- (`KismetMathLibrary.RandomFloat`) 0.5) _returnvalue) (* (- (`KismetMathLibrary.RandomFloat`) 0.5) _returnvalue))))
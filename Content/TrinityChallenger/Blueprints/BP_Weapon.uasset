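; BP_Weapon is a pickup weapon actor that attaches to the player character on overlap and fires on input.
; The first overlap with the BP_ThirdPersonCharacter snaps it to the owning actor of WeaponPos and zeroes its world rotation.
; It enables input on BeginPlay, regardless of pickup, and PrimaryAction passes a shoot flag and the Arrow's relative location to its Disparador component.
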(event `self.ReceiveBeginPlay`
  (bind _returnvalue (`GameplayStatics.GetPlayerController` 0))
  ;[1 1 1] Establecer input
  (`self.EnableInput` _returnvalue)
  (set `PlayerController.bEnableClickEvents` true _returnvalue))

(event `InputAction|PrimaryAction`
  (params (Key :type "Key Structure"))
  (bind _returnvalue (`self.GetComponentByClass` "/Game/TrinityChallenger/Blueprints/Disparador.Disparador_C"))
  ;[1 1 1] Disparar Arma
  (:`Pressed`
    (set `/Game/TrinityChallenger/Blueprints/Disparador.Shoot` true _returnvalue)
    (set `/Game/TrinityChallenger/Blueprints/Disparador.ShootPosition` (.location (`SceneComponent.GetRelativeTransform` (`self.Arrow`))) _returnvalue)))

(event `self.ReceiveActorBeginOverlap`
  (params (OtherActor :type "Actor Object Reference"))
  ;[1 1 1] Recoger Arma
  (if (not (`self.wasPickedUp`))
    (bind _returnvalue (`GameplayStatics.GetActorOfClass` "/Game/ThirdPerson/Blueprints/BP_ThirdPersonCharacter.BP_ThirdPersonCharacter_C"))
    (if (== _returnvalue OtherActor)
      (set `self.wasPickedUp` true)
      (`self.K2_AttachToActor` (`ActorComponent.GetOwner` (`/Game/ThirdPerson/Blueprints/BP_ThirdPersonCharacter.WeaponPos` _returnvalue)) "None" "SnapToTarget" "SnapToTarget" "KeepWorld")
      (`self.K2_SetActorRotation` (struct) true))))

(fn `UserConstructionScript`)
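; BP_AudioStarter plays an analyzed sound and drives audio-reactive visuals in sync with it.
; Construction takes the sound and duration from a LoudnessAnalyzer; playback waits until the StartPlay flag is set, then starts at reduced volume.
; Each playback-percent callback converts progress to seconds, samples precomputed normalized loudness on channel 0, and writes it to the Intensity of AudioVisualizer components on PostProcessVolumes.
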(event `self.ReceiveTick`
  (params (DeltaSeconds :type "Float (single-precision)"))
  (if (`self.startPlay`)
    (`AudioComponent.Play` (`self.Audio`) 0.0)
    (`AudioComponent.AdjustVolume` (`self.Audio`) 0.0 0.3 "Linear")
    (set `self.startPlay` false)))

(event `self.ReceiveBeginPlay`
  (add `AudioComponent.OnAudioPlaybackPercent` (`self.Audio`) (delegate `PlaybackPercentEvent`))
  (`AudioComponent.Stop` (`self.Audio`)))

(event `PlaybackPercentEvent`
  (params (PlayingSoundWave :type "SoundWave Object Reference") (PlaybackPercent :type "Float (single-precision)"))
  (bind _outactors (`GameplayStatics.GetAllActorsOfClass` "/Script/Engine.PostProcessVolume"))
  (for _array_element _outactors
    (bind _returnvalue (`self.GetComponentByClass` _array_element "/Game/TrinityChallenger/Blueprints/AudioVisualizer.AudioVisualizer_C"))
    (`/Engine/EditorBlueprintResources/StandardMacros.IsValid` _returnvalue
      (:`Is Valid`
        (set `/Game/TrinityChallenger/Blueprints/AudioVisualizer.Intensity` (`LoudnessNRT.GetNormalizedChannelLoudnessAtTime` (`self.LoudnessAnalyzer`) (* PlaybackPercent (`self.Duration`)) 0) _returnvalue)))))

(fn `UserConstructionScript`
  (bind _sound (`AudioAnalyzerNRT.Sound` (`self.LoudnessAnalyzer`)))
  (`AudioComponent.SetSound` (`self.Audio`) _sound)
  (set `self.Duration` (`SoundBase.Duration` _sound)))